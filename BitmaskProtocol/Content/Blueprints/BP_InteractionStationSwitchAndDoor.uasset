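; Interaction station pairing a switch with a door, which players open by completing a timed interaction and NPCs open by proximity.
; InteractionTrigger registers the station with the player while it is closed or open, CanInteract allows use only when closed, and Tick opens it once interaction time is reached.
; AITrigger tracks NPC capsules, closing the door when the last leaves.
; Separate open/close timelines lerp from the current position; construction previews IsOpen.
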(event OnComponentBeginOverlap(InteractionTrigger)
  (params (OverlappedComponent :type Primitive%20Component%20Object%20Reference) (OtherActor :type Actor%20Object%20Reference) (OtherComp :type Primitive%20Component%20Object%20Reference) (OtherBodyIndex :type Integer) (bFromSweep :type Boolean) (SweepResult :type Hit%20Result%20Structure%20%28by%20ref%29))
  (bind _asbp_player_character (Utilities|Casting|CastToBP_PlayerCharacter OtherActor))
  (Default|AddInteractingActor _asbp_player_character self))

(event OnComponentEndOverlap(InteractionTrigger)
  (params (OverlappedComponent :type Primitive%20Component%20Object%20Reference) (OtherActor :type Actor%20Object%20Reference) (OtherComp :type Primitive%20Component%20Object%20Reference) (OtherBodyIndex :type Integer))
  (bind _asbp_player_character (Utilities|Casting|CastToBP_PlayerCharacter OtherActor))
  (Default|RemoveInteractingActor _asbp_player_character self))

(event OnComponentBeginOverlap(AITrigger)
  (params (OverlappedComponent :type Primitive%20Component%20Object%20Reference) (OtherActor :type Actor%20Object%20Reference) (OtherComp :type Primitive%20Component%20Object%20Reference) (OtherBodyIndex :type Integer) (bFromSweep :type Boolean) (SweepResult :type Hit%20Result%20Structure%20%28by%20ref%29))
  (bind _asbp_npc_base (Utilities|Casting|CastToBP_NPC_Base OtherActor))
  (Utilities|Casting|CastToCapsuleComponent OtherComp)
  (CallFunction|OpenDoor)
  (Utilities|Array|AddUnique (Variables|Default|GetAs%20BP%20NPC%20Base) _asbp_npc_base))

(event OnComponentEndOverlap(AITrigger)
  (params (OverlappedComponent :type Primitive%20Component%20Object%20Reference) (OtherActor :type Actor%20Object%20Reference) (OtherComp :type Primitive%20Component%20Object%20Reference) (OtherBodyIndex :type Integer))
  (bind _as_bp_npc_base (Variables|Default|GetAs%20BP%20NPC%20Base))
  (bind _asbp_npc_base (Utilities|Casting|CastToBP_NPC_Base OtherActor))
  (Utilities|Casting|CastToCapsuleComponent OtherComp)
  (Utilities|Array|RemoveItem _as_bp_npc_base _asbp_npc_base)
  (if (Utilities|Array|IsEmpty _as_bp_npc_base)
    (CallFunction|CloseDoor)))

(event Custom|OpenDoor
  (bind _door (Variables|Default|GetDoor))
  (bind _door_2 (Variables|Default|GetDoor))
  (bind _closedlocation (Variables|Default|GetClosedLocation))
  (bind _openlocation (Variables|Default|GetOpenLocation))
  (if (not (Variables|Default|GetIsOpen))
    (Variables|Default|SetIsOpen true)
    (Utilities|FlowControl|Sequence
      (:then_0
        (bind _newtrack_0 (Timeline|Timeline_0 Stop)
          (:Update
            (Transformation|SetRelativeLocation _door (Math|Vector|Lerp(Vector) (Variables|/Script/Engine.SceneComponent|GetRelativeLocation _door) _closedlocation _newtrack_0) false false))
          (:Finished
            (Transformation|SetRelativeLocation _door _closedlocation false false))))
      (:then_1
        (bind _newtrack_0_2 (Timeline|Timeline PlayFromStart)
          (:Update
            (Transformation|SetRelativeLocation _door_2 (Math|Vector|Lerp(Vector) (Variables|/Script/Engine.SceneComponent|GetRelativeLocation _door_2) _openlocation _newtrack_0_2) false false))
          (:Finished
            (Transformation|SetRelativeLocation _door_2 _openlocation false false)))))))

(event Custom|CloseDoor
  (bind _door (Variables|Default|GetDoor))
  (bind _door_2 (Variables|Default|GetDoor))
  (bind _closedlocation (Variables|Default|GetClosedLocation))
  (bind _openlocation (Variables|Default|GetOpenLocation))
  (if (Variables|Default|GetIsOpen)
    (Variables|Default|SetIsOpen false)
    (Utilities|FlowControl|Sequence
      (:then_0
        (bind _newtrack_0 (Timeline|Timeline Stop)
          (:Update
            (Transformation|SetRelativeLocation _door_2 (Math|Vector|Lerp(Vector) (Variables|/Script/Engine.SceneComponent|GetRelativeLocation _door_2) _openlocation _newtrack_0) false false))
          (:Finished
            (Transformation|SetRelativeLocation _door_2 _openlocation false false))))
      (:then_1
        (bind _newtrack_0_2 (Timeline|Timeline_0 PlayFromStart)
          (:Update
            (Transformation|SetRelativeLocation _door (Math|Vector|Lerp(Vector) (Variables|/Script/Engine.SceneComponent|GetRelativeLocation _door) _closedlocation _newtrack_0_2) false false))
          (:Finished
            (Transformation|SetRelativeLocation _door _closedlocation false false)))))))

(event EventBeginPlay
  (|CallParentFunction) ; This node is disabled and will not be called.\nDrag off pins to build functionality.
)

(event Collision|EventActorBeginOverlap
  (params (OtherActor :type Actor%20Object%20Reference))
  (|CallParentFunction OtherActor) ; This node is disabled and will not be called.\nDrag off pins to build functionality.
)

(event EventTick
  (params (DeltaSeconds :type Float%20%28single-precision%29))
  (|CallParentFunction DeltaSeconds)
  (if (>= (Variables|Default|GetCurrentInteractionTime) (Variables|Default|GetInteractionTimeToOpen))
    (CallFunction|OpenDoor)))

(fn ConstructionScript
  (|CallParentFunction)
  (Transformation|SetRelativeLocation (Variables|Default|GetDoor) (select (Variables|Default|GetIsOpen) (Variables|Default|GetOpenLocation) (Variables|Default|GetClosedLocation)) false false))

(fn CanInteract
  (params (Character :type BP%20Player%20Character%20Object%20Reference))
  (bind _caninteract (|CallParentFunction Character))
  (return (and _caninteract (not (Variables|Default|GetIsOpen)))))