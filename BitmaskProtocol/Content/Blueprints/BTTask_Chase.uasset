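; Behavior tree task that makes an NPC AI controller chase a location stored in a blackboard key.
; On execute it casts the owner to AI_ControllerNPC, starts a navigation-projected move, and fails the task if that move fails.
; Each tick it reissues the move to the current key value to follow a changing target.
; It finishes successfully only when already at the goal with FinishAtGoal enabled.
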(event EventReceiveTickAI
  (params (OwnerController :type AI%20Controller%20Object%20Reference) (ControlledPawn :type Pawn%20Object%20Reference) (DeltaSeconds :type Float%20%28single-precision%29))
  (bind _as_ai_controller_npc (Variables|Default|GetAs%20AI%20Controller%20NPC))
  (Utilities|IsValid _as_ai_controller_npc
    (:Is%20Valid
      (bind _returnvalue (AI|Navigation|MovetoLocation _as_ai_controller_npc (Class|BTFunctionLibrary|GetBlackboardValueasVector (Variables|Default|GetTargetLocationKey)) -1.0 true true true true 0))
      (if (and (Utilities|Enum|Equal(Enum) _returnvalue "AlreadyAtGoal") (Variables|Default|GetFinishAtGoal))
        (AI|BehaviorTree|FinishExecute true)))))

(event EventReceiveExecuteAI
  (params (OwnerController :type AI%20Controller%20Object%20Reference) (ControlledPawn :type Pawn%20Object%20Reference))
  (bind _asai_controller_npc (Utilities|Casting|CastToAI_ControllerNPC OwnerController))
  (bind _output_get (Variables|Default|SetAs%20AI%20Controller%20NPC _asai_controller_npc))
  (bind _returnvalue (AI|Navigation|MovetoLocation _output_get (Class|BTFunctionLibrary|GetBlackboardValueasVector (Variables|Default|GetTargetLocationKey)) -1.0 true true true true 0))
  (if (Utilities|Enum|Equal(Enum) _returnvalue "Failed")
    (AI|BehaviorTree|FinishExecute false)))