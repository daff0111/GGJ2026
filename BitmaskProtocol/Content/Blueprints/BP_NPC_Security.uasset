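; Security guard NPC that detects the player by their current identity and arrests them on contact when aggressive.
; Each tick, while Calm or Alert, local suspicion rises for one specific perceived identity and otherwise drains, raising Alert and notifying BitmaskGameMode when full.
; Alert or Searching guards turn Aggressive on seeing the game mode's last known identity, and drop to Searching on losing the player.
; State changes set walk speed; capsule overlap while Aggressive triggers a one-time arrest.
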(event OnComponentBeginOverlap(Capsule)
  (params (OverlappedComponent :type Primitive%20Component%20Object%20Reference) (OtherActor :type Actor%20Object%20Reference) (OtherComp :type Primitive%20Component%20Object%20Reference) (OtherBodyIndex :type Integer) (bFromSweep :type Boolean) (SweepResult :type Hit%20Result%20Structure%20%28by%20ref%29))
  (if (Utilities|Enum|Equal(Enum) (Variables|Default|GetAlertLevel) "NewEnumerator3")
    (if (== OtherActor (Variables|Default|GetPerceivedPlayer))
      (CallFunction|Arrest))))

(event Custom|Arrest
  (Utilities|FlowControl|DoOnce false
    (:Completed
      (Default|Arrested (Variables|Default|GetPerceivedPlayer))
      (Animation|Montage|MontagePlay (Variables|Default|GetAnimInstance) "/Game/Characters/Mannequins/Anims/Rifle/MF_Rifle_Idle_ADS_Montage.MF_Rifle_Idle_ADS_Montage" 0.0 "MontageLength" 0.0 true))))

(event EventBeginPlay)

(event Collision|EventActorBeginOverlap
  (params (OtherActor :type Actor%20Object%20Reference)))

(event EventTick
  (params (DeltaSeconds :type Float%20%28single-precision%29))
  (|CallParentFunction DeltaSeconds)
  (CallFunction|UpdateSecuritySuspicion DeltaSeconds))

(fn ConstructionScript
  (|CallParentFunction))

(fn UpdateSecuritySuspicion
  (params (InputPin :type Float%20%28single-precision%29))
  (bind _maxlocalsuspicion (Variables|Default|GetMaxLocalSuspicion))
  (bind _perceivedplayer (Variables|Default|GetPerceivedPlayer))
  (bind _perceivedplayer_2 (Variables|Default|GetPerceivedPlayer))
  (bind _returnvalue (Utilities|IsValid _perceivedplayer_2))
  (Utilities|FlowControl|Sequence
    (:then_0
      (switch Utilities|FlowControl|Switch|SwitchonEAlertState (Variables|Default|GetAlertLevel)
        (:NewEnumerator0
          _)
        (:NewEnumerator1
          _))
      (Utilities|IsValid _perceivedplayer
        (:Is%20Valid
          (if (Utilities|Enum|Equal(Enum) (Variables|/Game/Blueprints/BP_PlayerCharacter.BP_PlayerCharacter_C|GetCurrentIdentity _perceivedplayer) "NewEnumerator0")
            (bind _output_get (Variables|Default|SetLocalSuspicion (Math|Float|Min(Float) (+ (Variables|Default|GetLocalSuspicion) (* InputPin (Variables|Default|GetSuspicionRaiseRate))) _maxlocalsuspicion)))
            (if (>= _output_get _maxlocalsuspicion)
              (CallFunction|SetAlertState "NewEnumerator1")
              (Default|RaiseAlertLevel (Variables|Default|GetBitmask%20Game%20Mode) 2)
              (Default|SetLastPlayerLocation (Variables|Default|GetBitmask%20Game%20Mode) (Transformation|GetActorLocation (Variables|Default|GetPerceivedPlayer))))
            (else
              (bind _output_get_2 (Variables|Default|SetLocalSuspicion (Math|Float|Max(Float) (- (Variables|Default|GetLocalSuspicion) (* InputPin (Variables|Default|GetSuspicionDrainRate))) 0.0) :!label _label))
              (if (and (<= _output_get_2 0.0) (Utilities|Enum|Equal(Enum) (Variables|Default|GetAlertLevel) "NewEnumerator1"))
                (CallFunction|SetAlertState "NewEnumerator0")))))
        (:Is%20Not%20Valid
          (goto _label))))
    (:then_1
      (switch Utilities|FlowControl|Switch|SwitchonEAlertState (Variables|Default|GetAlertLevel)
        (:NewEnumerator1
          (if _returnvalue :!label _label_2
            (if (Utilities|Enum|Equal(Enum) (Variables|/Game/Blueprints/BP_PlayerCharacter.BP_PlayerCharacter_C|GetCurrentIdentity _perceivedplayer_2) (Variables|/Game/Blueprints/BP_BitmaskGameMode.BP_BitmaskGameMode_C|GetLastPlayerIdentity (Variables|Default|GetBitmask%20Game%20Mode)))
              (CallFunction|SetAlertState "NewEnumerator3"))))
        (:NewEnumerator2
          (goto _label_2))
        (:NewEnumerator3
          (if (not _returnvalue)
            (CallFunction|SetAlertState "NewEnumerator2")))))))

(fn SetAlertState
  (params (AlertLevel :type EAlertState%20Enum :default "NewEnumerator0"))
  (bind _output_get (Variables|Default|SetAlertLevel AlertLevel))
  (Variables|/Script/Engine.CharacterMovementComponent|SetMaxWalkSpeed (Variables|Character|GetCharacterMovement) (Utilities|Select :Index _output_get :NewEnumerator0 3e+02 :NewEnumerator1 3e+02 :NewEnumerator2 3.5e+02 :NewEnumerator3 4e+02))
  (switch Utilities|FlowControl|Switch|SwitchonEAlertState _output_get
    (:NewEnumerator2
      _)
    (:NewEnumerator3
      (if (Collision|IsOverlappingActor (Variables|Default|GetCapsule) (Variables|Default|GetPerceivedPlayer) :!class /Script/Engine.PrimitiveComponent)
        (CallFunction|Arrest))))
  (Variables|Default|SetLocalSuspicion (Variables|Default|GetMaxLocalSuspicion)))