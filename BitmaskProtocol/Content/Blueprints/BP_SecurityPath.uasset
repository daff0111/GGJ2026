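; BP_SecurityPath is a spline-based path actor that displays its route as a closed loop of spline meshes.
; The construction script creates a movable, uniformly configured mesh segment between each pair of neighboring spline points, plus one joining last to first.
; Segments are positioned by endpoints only, without setting tangents, and stored in Meshes.
; SetVisible shows or hides all stored segments; the event graph is empty.
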(event EventBeginPlay)

(event Collision|EventActorBeginOverlap
  (params (OtherActor :type Actor%20Object%20Reference)))

(event EventTick
  (params (DeltaSeconds :type Float%20%28single-precision%29)))

(fn ConstructionScript
  (bind _spline (Variables|Default|GetSpline))
  (bind _returnvalue (Spline|GetNumberOfSplinePoints _spline))
  (Utilities|Array|Clear (Variables|Default|GetMeshes))
  (for _index (range 0 (- _returnvalue 2))
    (CallFunction|CreateSplineMesh (.position (Spline|GetSplinePointAt _spline _index "Local")) (.position (Spline|GetSplinePointAt _spline (+ _index 1) "Local"))))
  (CallFunction|CreateSplineMesh (.position (Spline|GetSplinePointAt _spline (- _returnvalue 1) "Local")) (.position (Spline|GetSplinePointAt _spline 0 "Local"))))

(fn CreateSplineMesh
  (params (StartPos :type Vector) (EndPos :type Vector))
  (bind _splinescale (Variables|Default|GetSplineScale))
  (bind _returnvalue (AddComponent|AddSplineMeshComponent false (Math|Transform|MakeTransform "0, 0, 0" "0.000000,0.000000,0.000000" "1.000000,1.000000,1.000000")))
  (SplineMesh|SetStartScale _returnvalue _splinescale true :!class /Script/Engine.SplineMeshComponent)
  (SplineMesh|SetEndScale _returnvalue _splinescale true :!class /Script/Engine.SplineMeshComponent)
  (Transformation|SetMobility _returnvalue "Movable")
  (SplineMesh|SetStartPosition _returnvalue StartPos true)
  (SplineMesh|SetEndPosition _returnvalue EndPos true)
  (Utilities|Array|Add (Variables|Default|GetMeshes) _returnvalue))

(fn SetVisible
  (params (bNewVisibility :type Boolean))
  (for _array_element (Variables|Default|GetMeshes)
    (Rendering|SetVisibility _array_element bNewVisibility true)))