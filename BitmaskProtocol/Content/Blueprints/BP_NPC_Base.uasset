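; Base NPC Blueprint that the player character can sample, with an identity role shown through its color.
; The construction script creates dynamic materials for two mesh slots, tints them by identity and sizes the sphere from the sampling radius.
; Sphere overlaps add or remove the NPC as a sampling actor on the player.
; Start and complete sampling events are empty, and the sampling check always returns true.
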(event OnComponentBeginOverlap(Sphere)
  (params (OverlappedComponent :type Primitive%20Component%20Object%20Reference) (OtherActor :type Actor%20Object%20Reference) (OtherComp :type Primitive%20Component%20Object%20Reference) (OtherBodyIndex :type Integer) (bFromSweep :type Boolean) (SweepResult :type Hit%20Result%20Structure%20%28by%20ref%29))
  ;[0.15 0.15 0.15 0.5] Sampling
  (bind _asbp_player_character (Utilities|Casting|CastToBP_PlayerCharacter OtherActor))
  (Default|AddSamplingActor _asbp_player_character self))

(event OnComponentEndOverlap(Sphere)
  (params (OverlappedComponent :type Primitive%20Component%20Object%20Reference) (OtherActor :type Actor%20Object%20Reference) (OtherComp :type Primitive%20Component%20Object%20Reference) (OtherBodyIndex :type Integer))
  ;[0.15 0.15 0.15 0.5] Sampling
  (bind _asbp_player_character (Utilities|Casting|CastToBP_PlayerCharacter OtherActor))
  (Default|RemoveSamplingActor _asbp_player_character self))

(event EventCompleteSampling
  (params (Identity :type EIdentityType%20Enum :default "NewEnumerator0")))

(event EventStartSampling
  (params (Requester :type Actor%20Object%20Reference)))

(fn ConstructionScript
  (bind _mesh (Variables|Character|GetMesh))
  (bind _mymaterials (Variables|Default|GetMyMaterials))
  (Utilities|FlowControl|Sequence
    (:then_0
      (bind _returnvalue (Rendering|Material|CreateDynamicMaterialInstance _mesh 0 0 "None" :!class /Script/Engine.PrimitiveComponent))
      (Utilities|Array|Add _mymaterials _returnvalue))
    (:then_1
      (bind _returnvalue_2 (Rendering|Material|CreateDynamicMaterialInstance _mesh 1 0 "None" :!class /Script/Engine.PrimitiveComponent))
      (Utilities|Array|Add _mymaterials _returnvalue_2))
    (:then_2
      (CallFunction|UpdateMaterials (Variables|Default|GetIdentity)))
    (:then_3
      (Components|Sphere|SetSphereRadius (Variables|Default|GetSphere) (Variables|Default|GetSamplingRadius) true))))

(fn UpdateMaterials
  (params (CurrentIdentity :type EIdentityType%20Enum :default "NewEnumerator0"))
  (Rendering|Material|SetVectorParameterValue (Variables|Default|GetMyMaterials) "Paint Tint" (Utilities|Select :Index CurrentIdentity :NewEnumerator0 "(R=1.000000,G=1.000000,B=1.000000,A=1.000000)" :NewEnumerator1 "(R=0.000000,G=0.472568,B=1.000000,A=1.000000)" :NewEnumerator2 "(R=1.000000,G=0.013193,B=0.000000,A=1.000000)" :NewEnumerator3 "(R=1.000000,G=0.885625,B=0.000000,A=1.000000)" :NewEnumerator4 "(R=0.562971,G=0.000000,B=1.000000,A=1.000000)") :!class /Script/Engine.MaterialInstanceDynamic))

(fn CanSample
  (return true))