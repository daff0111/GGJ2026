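; Twin-stick player character that samples nearby NPCs to copy their identity, shown as mesh tint and in an identity widget.
; A looping timer drains identity time, scaled by sprint while moving, and picks the closest NPC and interaction station for hold-input actions.
; Identity expiry clears the disguise and plays a time-dilation Timeline.
; Tick handles mouse or stick facing, animation and debug prints until arrest disables input.
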(event Custom|Reset%20Item
  ;[0.15 0.15 0.15 0.502] If the Player has a smart bomb, fire it when the Use Item input action is called.
  (Utilities|FlowControl|DoOnce false ; enters at Reset
    (:Completed
      (Utilities|FlowControl|Sequence
        (:then_0
          (Game|SpawnActorfromClass "/Game/Prototypes/Variant_TwinStick/Blueprints/BP_TwinStickAoEAttack.BP_TwinStickAoEAttack_C" (Math|Conversions|ToTransform(Vector) (Transformation|GetActorLocation)) "Undefined" "MultiplyWithRoot" 0 0)
          (Utilities|FlowControl|Delay 1.0)
          (CallFunction|ResetItem))
        (:then_1
          (Math|Integer|DecrementInt (Variables|Gameplay|GetItems)
            (:%20%20
              (Class|BPITwinstick|ItemUsed(Message) (Game|GetGameMode) (Variables|Gameplay|GetItems)))))))))

(event Custom|Arrested
  ;[0.15 0.04664 0.04793 0.5] Arrest
  (CallFunction|PerformArrest))

(event Custom|EventUpdateTimer
  ;[0.15 0.15 0.15 0.502] Player Rotation is handled on Tick
  (Identity|UpdateIdentityTime (Variables|Identity|GetTimerInterval))
  (Sampling|UpdateClosestActor)
  (Interaction|UpdateClosestInteraction))

(event Custom|BitmaskLost
  ;[0.15 0.15 0.15 0.502] Dilate Time via a Timeline
  (Variables|/Game/UI/UI_BitmaskIdentity.UI_BitmaskIdentity_C|SetBitmaskLost (Variables|Default|GetUI%20Bitmask%20Identity) true)
  (bind _timedilation (Timeline|Timeline Play)
    (:Update
      (Utilities|Time|SetGlobalTimeDilation _timedilation))
    (:Finished
      (Utilities|Time|SetGlobalTimeDilation 1.0)
      (Variables|/Game/UI/UI_BitmaskIdentity.UI_BitmaskIdentity_C|SetBitmaskLost (Variables|Default|GetUI%20Bitmask%20Identity) false))))

(event Input|EnhancedActionEvents|EnhancedInputActionIA_Action_Move
  (params (ActionValue :type Vector%202D%20Structure) (ElapsedSeconds :type Float%20%28double-precision%29) (TriggeredSeconds :type Float%20%28double-precision%29) (InputAction :type Input%20Action%20Object%20Reference :default "/Game/Prototypes/Variant_TwinStick/Input/Actions/IA_Action_Move.IA_Action_Move"))
  ;[0.15 0.15 0.15 0.502] Move the Player and control their aiming direction if on a Gamepad
  (Variables|Controls|SetLast%20Move (Math|Vector2D|MakeVector2D (.x ActionValue) (.y ActionValue)))
  (Input|Move (.x ActionValue) (.y ActionValue)))

(event Input|EnhancedActionEvents|EnhancedInputActionIA_Action_StickAim
  (params (ActionValue :type Vector%202D%20Structure) (ElapsedSeconds :type Float%20%28double-precision%29) (TriggeredSeconds :type Float%20%28double-precision%29) (InputAction :type Input%20Action%20Object%20Reference :default "/Game/Prototypes/Variant_TwinStick/Input/Actions/IA_Action_StickAim.IA_Action_StickAim"))
  ;[0.15 0.15 0.15 0.502] Move the Player and control their aiming direction if on a Gamepad
  (Input|StickAim (.x ActionValue) (.y ActionValue)))

(event Input|EnhancedActionEvents|EnhancedInputActionIA_Action_MouseAim
  (params (ActionValue :type Vector%202D%20Structure) (ElapsedSeconds :type Float%20%28double-precision%29) (TriggeredSeconds :type Float%20%28double-precision%29) (InputAction :type Input%20Action%20Object%20Reference :default "/Game/Prototypes/Variant_TwinStick/Input/Actions/IA_Action_MouseAim.IA_Action_MouseAim"))
  ;[0.15 0.15 0.15 0.502] If Player moves the mouse, enable mouse controls.
  (Variables|/Script/Engine.PlayerController|SetbShowMouseCursor (Game|GetPlayerController 0) true))

(event Input|EnhancedActionEvents|EnhancedInputActionIA_Action_UseItem
  (params (ActionValue :type Boolean) (ElapsedSeconds :type Float%20%28double-precision%29) (TriggeredSeconds :type Float%20%28double-precision%29) (InputAction :type Input%20Action%20Object%20Reference :default "/Game/Prototypes/Variant_TwinStick/Input/Actions/IA_Action_UseItem.IA_Action_UseItem"))
  ;[0.15 0.15 0.15 0.502] If the Player has a smart bomb, fire it when the Use Item input action is called.
  (if (> (Variables|Gameplay|GetItems) 0)
    _))

(event Input|EnhancedActionEvents|EnhancedInputActionIA_Action_Dash
  (params (ActionValue :type Boolean) (ElapsedSeconds :type Float%20%28double-precision%29) (TriggeredSeconds :type Float%20%28double-precision%29) (InputAction :type Input%20Action%20Object%20Reference :default "/Game/Prototypes/Variant_TwinStick/Input/Actions/IA_Action_Dash.IA_Action_Dash"))
  ;[0.15 0.15 0.15 0.502] Sprint
  (:Triggered
    (Variables|Controls|SetSprint 1.0))
  (:Canceled
    (Variables|Controls|SetSprint 0.5 :!label _label))
  (:Completed
    (goto _label)))

(event Input|EnhancedActionEvents|EnhancedInputActionIA_Action_Sample
  (params (ActionValue :type Boolean) (ElapsedSeconds :type Float%20%28double-precision%29) (TriggeredSeconds :type Float%20%28double-precision%29) (InputAction :type Input%20Action%20Object%20Reference :default "/Game/Prototypes/Variant_TwinStick/Input/Actions/IA_Action_Sample.IA_Action_Sample"))
  ;[0.15 0.15 0.15 0.5] Sampling
  (:Triggered
    (Sampling|ContinueSampling ElapsedSeconds))
  (:Started
    (CallFunction|StartSampling (Variables|Sampling|GetClosestNPC)))
  (:Canceled
    (CallFunction|StopSampling :!label _label))
  (:Completed
    (goto _label)))

(event Input|EnhancedActionEvents|EnhancedInputActionIA_Action_Interact
  (params (ActionValue :type Boolean) (ElapsedSeconds :type Float%20%28double-precision%29) (TriggeredSeconds :type Float%20%28double-precision%29) (InputAction :type Input%20Action%20Object%20Reference :default "/Game/Prototypes/Variant_TwinStick/Input/Actions/IA_Action_Interact.IA_Action_Interact"))
  ;[0.15 0.15 0.15 0.5] Sampling
  (:Started
    (Interaction|StartInteracting))
  (:Canceled
    (Interaction|StopInteracting :!label _label))
  (:Completed
    (goto _label)))

(event EventTick
  (params (DeltaSeconds :type Float%20%28single-precision%29))
  ;[0.15 0.15 0.15 0.502] Player Rotation is handled on Tick
  (if (not (Variables|Default|GetIsArrested))
    (Utilities|FlowControl|Sequence
      (:then_0
        (Input|UpdateRotation))
      (:then_1
        (CallFunction|UpdateAnimation))
      (:then_3
        (CallFunction|DebugPrint)))))

(event EventStopSampling
  ;[0.15 0.15 0.15 0.5] Sampling
  (Sampling|StopSamplingNPC))

(event EventBeginPlay
  ;[0.1432 0.7656 0.1632 0.502] Begin Play
  (Utilities|FlowControl|Sequence
    (:then_0
      (Utilities|Time|SetTimerbyEvent (EventDispatchers|CreateEvent :!event Custom|EventUpdateTimer) (Variables|Identity|GetTimerInterval) true))
    (:then_1
      (Input|AddMappingContext (PlayerController|LocalPlayerSubsystems|GetEnhancedInputLocalPlayerSubsystem (Game|GetPlayerController 0)) "/Game/Prototypes/Variant_TwinStick/Input/IMC_TwinStick.IMC_TwinStick" 0 "(bIgnoreAllPressedKeysUntilRelease=True,bForceImmediately=False,bNotifyUserSettings=False)"))
    (:then_2
      (bind _asabp_unarmed (Utilities|Casting|CastToABP_Unarmed (Components|SkeletalMesh|GetAnimInstance (Variables|Character|GetMesh))))
      (Variables|Components|SetAnimInstance _asabp_unarmed))
    (:then_3
      (bind _asui_bitmask_identity (Utilities|Casting|CastToUI_BitmaskIdentity (UserInterface|GetWidget (Variables|Default|GetIdentityMaskWidget))))
      (Variables|Default|SetUI%20Bitmask%20Identity _asui_bitmask_identity))
    (:then_4
      (Identity|UpdateIdentity "NewEnumerator0"))
    (:then_5
      (bind _asbp_bitmask_game_mode (Utilities|Casting|CastToBP_BitmaskGameMode (Game|GetGameMode)))
      (Variables|Default|SetBitmask%20Game%20Mode _asbp_bitmask_game_mode))))

(event EventStartSampling
  (params (Requester :type Actor%20Object%20Reference))
  ;[0.15 0.15 0.15 0.5] Sampling
  (Sampling|StartSamplingNPC Requester))

(event EventInteraction
  (params (Interactor :type Actor%20Object%20Reference))
  ;[0.15 0.15 0.15 0.502] If an Item sends an interaction message to the Player, add an Item to the inventory
  (if (== (Utilities|GetClass Interactor) "/Game/Prototypes/Variant_TwinStick/Blueprints/BP_TwinStickPickup.BP_TwinStickPickup_C")
    (Math|Integer|IncrementInt (Variables|Gameplay|GetItems)
      (:%20%20
        ;[0.15 0.15 0.15 0.502] If the Player has a smart bomb, fire it when the Use Item input action is called.
        (Class|BPITwinstick|ItemUsed(Message) (Game|GetGameMode) (Variables|Gameplay|GetItems))))))

(event EventProjectileImpact
  (params (ForwardVector :type Vector :default "0, 0, 0"))
  ;[0.15 0.15 0.15 0.502] Knock Back Player
  (Character|LaunchCharacter (* (Math|Vector|MakeVector (.x ForwardVector) (.y ForwardVector) 0.0) (Variables|Gameplay|GetKnockbackStrength)) true true))

(event EventPrimaryThumbstick
  (params (Axis :type Vector%202D%20Structure))
  ;[0.15 0.15 0.15 0.502] Move the Player and control their aiming direction if on a Gamepad
  (Variables|Controls|SetLast%20Move (Math|Vector2D|MakeVector2D (.y Axis) (.x Axis)))
  (Input|Move (.y Axis) (.x Axis)))

(event EventTouchItemStart
  ;[0.15 0.15 0.15 0.502] If the Player has a smart bomb, fire it when the Use Item input action is called.
  (if (> (Variables|Gameplay|GetItems) 0)
    _))

(event EventSecondaryThumbstick
  (params (Axis :type Vector%202D%20Structure))
  ;[0.15 0.15 0.15 0.502] Move the Player and control their aiming direction if on a Gamepad
  (Input|TouchAim (.y Axis) (.x Axis)))

(fn ConstructionScript
  (bind _mesh (Variables|Character|GetMesh))
  (bind _mymaterials (Variables|Components|GetMyMaterials))
  (Utilities|FlowControl|Sequence
    (:then_0
      (bind _returnvalue (Rendering|Material|CreateDynamicMaterialInstance _mesh 0 0 "None" :!class /Script/Engine.PrimitiveComponent))
      (Utilities|Array|Add _mymaterials _returnvalue))
    (:then_1
      (bind _returnvalue_2 (Rendering|Material|CreateDynamicMaterialInstance _mesh 1 0 "None" :!class /Script/Engine.PrimitiveComponent))
      (Utilities|Array|Add _mymaterials _returnvalue_2))
    (:then_3
      (Identity|UpdateIdentity "NewEnumerator0"))))

(fn SnapPlayertoFacing
  (bind _returnvalue (Transformation|GetActorRotation))
  (bind _target_rotation (Variables|Controls|GetTarget%20Rotation))
  (Transformation|SetActorRotation (Math|Rotator|MakeRotator (.roll _returnvalue) (.pitch _returnvalue) (Math|Float|SelectFloat (Math|Float|Lerp (.yaw _returnvalue) _target_rotation 0.1) _target_rotation (< (Math|Float|Absolute(Float) (- (.yaw _returnvalue) _target_rotation)) 2e+02))))
  (return))

(fn RotatePlayer
  (bind _returnvalue (Transformation|GetActorRotation))
  (if (not (Math|Float|NearlyEqual(Float) (.yaw _returnvalue) (Variables|Controls|GetTarget%20Rotation) 0.5))
    (Transformation|SetActorRotation (Math|Rotator|MakeRotator (.roll _returnvalue) (.pitch _returnvalue) (.yaw (Math|Interpolation|RInterpTo (Transformation|GetActorRotation) (Math|Rotator|MakeRotator (.roll _returnvalue) (.pitch _returnvalue) (Variables|Controls|GetTarget%20Rotation)) (Utilities|Time|GetWorldDeltaSeconds) 1e+01))))
    (return)))

(fn Move
  (params (Axis%20X :type Float%20%28double-precision%29) (Axis%20Y :type Float%20%28double-precision%29))
  (bind _returnvalue (Pawn|GetControlRotation :!class /Script/Engine.Pawn))
  (bind _returnvalue_2 (Pawn|GetControlRotation :!class /Script/Engine.Pawn))
  (bind _sprint (Variables|Controls|GetSprint))
  (Pawn|Input|AddMovementInput (Math|Vector|GetForwardVector (Math|Rotator|MakeRotator (.roll _returnvalue) 0.0 (.yaw _returnvalue))) (* Axis%20X _sprint) false)
  (Pawn|Input|AddMovementInput (Math|Vector|GetRightVector (Math|Rotator|MakeRotator (.roll _returnvalue_2) 0.0 (.yaw _returnvalue_2))) (* Axis%20Y _sprint) false))

(fn StickAim
  (params (Axis%20X :type Float%20%28double-precision%29%20%28by%20ref%29) (Axis%20Y :type Float%20%28double-precision%29))
  (bind _result (Math|Float|NegateFloat Axis%20X)
    (:%20%20
      (Variables|Controls|SetTarget%20Rotation (Class|KismetMathLibrary|DegAtan2 Axis%20Y _result))
      (Variables|/Script/Engine.PlayerController|SetbShowMouseCursor (Game|GetPlayerController 0) false))))

(fn TouchAim
  (params (Axis%20X :type Float%20%28double-precision%29%20%28by%20ref%29) (Axis%20Y :type Float%20%28double-precision%29))
  (Variables|Controls|SetTarget%20Rotation (Class|KismetMathLibrary|DegAtan2 Axis%20Y Axis%20X))
  (Variables|/Script/Engine.PlayerController|SetbShowMouseCursor (Game|GetPlayerController 0) false))

(fn UpdateIdentity
  (params (CurrentIdentity :type EIdentityType%20Enum :default "NewEnumerator0"))
  (bind _ui_bitmask_identity (Variables|Default|GetUI%20Bitmask%20Identity))
  (bind _output_get (Variables|Identity|SetCurrentIdentity CurrentIdentity))
  (Rendering|Material|SetVectorParameterValue (Variables|Components|GetMyMaterials) "Paint Tint" (Utilities|Select :Index _output_get :NewEnumerator0 "(R=1.000000,G=1.000000,B=1.000000,A=1.000000)" :NewEnumerator1 "(R=0.000000,G=0.500000,B=1.000000,A=1.000000)" :NewEnumerator2 "(R=1.000000,G=0.013193,B=0.000000,A=1.000000)" :NewEnumerator3 "(R=1.000000,G=1.000000,B=0.000000,A=1.000000)" :NewEnumerator4 "(R=0.500000,G=0.000000,B=1.000000,A=1.000000)") :!class /Script/Engine.MaterialInstanceDynamic)
  (Utilities|IsValid _ui_bitmask_identity
    (:Is%20Valid
      (Variables|/Game/UI/UI_BitmaskIdentity.UI_BitmaskIdentity_C|SetPlayerIdentity _ui_bitmask_identity (Variables|Identity|GetCurrentIdentity)))))

(fn StartSamplingNPC
  (params (Actor :type Actor%20Object%20Reference))
  (bind _ui_bitmask_identity (Variables|Default|GetUI%20Bitmask%20Identity))
  (if (not (Variables|Sampling|GetIsSampling))
    (bind _asbp_npc_base (Utilities|Casting|CastToBP_NPC_Base Actor))
    (bind _cansample (Sampling|CanPerformSample _asbp_npc_base))
    (if _cansample
      (Variables|Sampling|SetIsSampling true)
      (bind _output_get (Variables|Sampling|SetSamplingNPC _asbp_npc_base))
      (Default|StartSampling _output_get self)
      (Variables|Sampling|SetCurrentSamplingTime 0.0)
      (Utilities|IsValid _ui_bitmask_identity
        (:Is%20Valid
          (Variables|/Game/UI/UI_BitmaskIdentity.UI_BitmaskIdentity_C|SetIsSampling _ui_bitmask_identity true)
          (Variables|/Game/UI/UI_BitmaskIdentity.UI_BitmaskIdentity_C|SetSamplingTime _ui_bitmask_identity 0.0)
          (Variables|/Game/UI/UI_BitmaskIdentity.UI_BitmaskIdentity_C|SetSamplingIdentity _ui_bitmask_identity (Variables|/Game/Blueprints/BP_NPC_Base.BP_NPC_Base_C|GetIdentity _output_get)))))))

(fn StopSamplingNPC
  (bind _ui_bitmask_identity (Variables|Default|GetUI%20Bitmask%20Identity))
  (Utilities|IsValid (Variables|Sampling|GetSamplingNPC)
    (:Is%20Valid
      (Default|StopSampling (Variables|Sampling|GetSamplingNPC))
      (Variables|Sampling|SetIsSampling false)
      (Variables|Sampling|SetSamplingNPC 0)
      (Variables|Sampling|SetCurrentSamplingTime 0.0)
      (Utilities|IsValid _ui_bitmask_identity
        (:Is%20Valid
          (Variables|/Game/UI/UI_BitmaskIdentity.UI_BitmaskIdentity_C|SetIsSampling _ui_bitmask_identity false)
          (Variables|/Game/UI/UI_BitmaskIdentity.UI_BitmaskIdentity_C|SetSamplingTime _ui_bitmask_identity 0.0))))))

(fn ContinueSampling
  (params (SamplingTime :type Float%20%28double-precision%29))
  (bind _samplingnpc (Variables|Sampling|GetSamplingNPC))
  (bind _ui_bitmask_identity (Variables|Default|GetUI%20Bitmask%20Identity))
  (bind _samplingnpc_2 (Variables|Sampling|GetSamplingNPC))
  (bind _identity (Variables|/Game/Blueprints/BP_NPC_Base.BP_NPC_Base_C|GetIdentity _samplingnpc))
  (if (Variables|Sampling|GetIsSampling)
    (Utilities|IsValid _samplingnpc_2
      (:Is%20Valid
        (bind _cansample (Sampling|CanPerformSample _samplingnpc_2))
        (if _cansample
          (bind _output_get (Variables|Sampling|SetCurrentSamplingTime SamplingTime))
          (if (> _output_get (Variables|/Game/Blueprints/BP_NPC_Base.BP_NPC_Base_C|GetSamplingTime _samplingnpc_2))
            (Default|CompleteSampling _samplingnpc _identity)
            (CallFunction|CompleteSampling _identity)
            (else
              (Utilities|IsValid _ui_bitmask_identity
                (:Is%20Valid
                  (Variables|/Game/UI/UI_BitmaskIdentity.UI_BitmaskIdentity_C|SetSamplingTime _ui_bitmask_identity (/ (Variables|Sampling|GetCurrentSamplingTime) (Variables|/Game/Blueprints/BP_NPC_Base.BP_NPC_Base_C|GetSamplingTime (Variables|Sampling|GetSamplingNPC))))))))
          (else
            (CallFunction|StopSampling :!label _label))))
      (:Is%20Not%20Valid
        (goto _label)))))

(fn AddSamplingActor
  (params (NewItem :type Actor%20Object%20Reference%20%28by%20ref%29))
  (Utilities|Array|AddUnique (Variables|Sampling|GetSamplingActors) NewItem))

(fn RemoveSamplingActor
  (params (NewItem :type Actor%20Object%20Reference%20%28by%20ref%29))
  (Utilities|Array|RemoveItem (Variables|Sampling|GetSamplingActors) NewItem)
  (if (== NewItem (Variables|Sampling|GetSamplingNPC))
    (CallFunction|StopSampling)))

(fn UpdateRotation
  (bind _returnvalue (Game|GetPlayerController 0))
  (bind _hitresult (Game|Player|GetHitResultUnderCursorbyChannel _returnvalue "TraceTypeQuery1" true))
  (bind (_bblockinghit _binitialoverlap _time _distance _location) (Collision|BreakHitResult _hitresult))
  (if (Variables|/Script/Engine.PlayerController|GetbShowMouseCursor (Game|GetPlayerController 0))
    (if _bblockinghit
      (Variables|Controls|SetTarget%20Rotation (.yaw (Math|Rotator|FindLookatRotation (Transformation|GetActorLocation) _location)))
      (CallFunction|SnapPlayertoFacing))
    (else
      (Input|RotatePlayer))))

(fn UpdateClosestActor
  (LocalVariables|SetMyLocation (Transformation|GetActorLocation))
  (LocalVariables|SetClosestDistanceSqr (LocalVariables|GetFLT_MAX))
  (for _array_element (Variables|Sampling|GetSamplingActors)
    (if (<= (Class|KismetMathLibrary|VectorDistanceSquared (Transformation|GetActorLocation _array_element) (LocalVariables|GetMyLocation)) (LocalVariables|GetClosestDistanceSqr))
      (LocalVariables|SetClosestDistanceSqr (Class|KismetMathLibrary|VectorDistanceSquared (Transformation|GetActorLocation _array_element) (LocalVariables|GetMyLocation)))
      (LocalVariables|SetClosestActor _array_element)))
  (Variables|Sampling|SetClosestNPC (LocalVariables|GetClosestActor)))

(fn CanPerformSample
  (params (NPC :type BP%20NPC%20Base%20Object%20Reference))
  (bind _cansample (Default|CanSample NPC))
  (return (and _cansample (Variables|Sampling|GetCanSample))))

(fn DebugPrint
  (bind _closestinteraction (Variables|Interaction|GetClosestInteraction))
  (bind _currentsamplingtime (Variables|Sampling|GetCurrentSamplingTime))
  (bind _closestnpc (Variables|Sampling|GetClosestNPC))
  (bind _currentidentitytime (Variables|Identity|GetCurrentIdentityTime))
  (Utilities|FlowControl|Sequence
    (:then_0
      (Utilities|IsValid _closestnpc
        (:Is%20Valid
          (Development|PrintString (Utilities|String|Append "Closest NPC: " (Utilities|GetDisplayName _closestnpc)) true true "(R=0.000000,G=0.660000,B=1.000000,A=1.000000)" 0.0))))
    (:then_1
      (if (> _currentsamplingtime 0.0)
        (Development|PrintString (Utilities|String|Append "Sampling Time: " (Utilities|String|ToString(Text) (Utilities|Text|ToText(Float) _currentsamplingtime "HalfToEven" false true 1 326 0 2))) true true "(R=0.930399,G=1.000000,B=0.209581,A=1.000000)" 0.0)))
    (:then_2
      (if (> _currentidentitytime 0.0)
        (Development|PrintString (Class|KismetStringLibrary|BuildStringDouble "Identity Time: " "" _currentidentitytime) true true "(R=1.000000,G=0.503576,B=0.053584,A=1.000000)" 0.0)))
    (:then_3
      (if (Variables|Interaction|GetIsInteracting)
        (Development|PrintString "Interacting" true true "(R=1.000000,G=0.098498,B=0.074143,A=1.000000)" 0.0)))
    (:then_4
      (Utilities|IsValid _closestinteraction
        (:Is%20Valid
          (Development|PrintString (Utilities|String|Append "Closest NPC: " (Utilities|GetDisplayName _closestinteraction)) true true "(R=0.000000,G=0.660000,B=1.000000,A=1.000000)" 0.0))))))

(fn UpdateIdentityTime
  (params (DeltaTime :type Float%20%28double-precision%29))
  (if (Utilities|Enum|NotEqual(Enum) (Variables|Identity|GetCurrentIdentity) "NewEnumerator0")
    (bind _output_get (Variables|Identity|SetCurrentIdentityTime (- (Variables|Identity|GetCurrentIdentityTime) (* DeltaTime (Variables|Identity|GetIdentityDrainRate) (select (> (Math|Vector|VectorLengthSquared (Transformation|GetVelocity)) 0.0) (* (Variables|Controls|GetSprint) 2.0) 1.0)))))
    (CallFunction|UpdateUITimer)
    (if (<= _output_get 0.0)
      (CallFunction|BitmaskLost)
      (Identity|UpdateIdentity "NewEnumerator0"))))

(fn AddInteractingActor
  (params (NewItem :type Actor%20Object%20Reference%20%28by%20ref%29))
  (Utilities|Array|AddUnique (Variables|Interaction|GetInteractingActors) NewItem))

(fn RemoveInteractingActor
  (params (NewItem :type Actor%20Object%20Reference%20%28by%20ref%29))
  (Utilities|Array|RemoveItem (Variables|Interaction|GetInteractingActors) NewItem)
  (if (== NewItem (Variables|Interaction|GetInteractingStation))
    (Interaction|StopInteracting)))

(fn StartInteracting
  (if (not (Variables|Sampling|GetIsSampling))
    (if (not (Variables|Interaction|GetIsInteracting))
      (bind _asbp_interaction_station_base (Utilities|Casting|CastToBP_InteractionStationBase (Variables|Interaction|GetClosestInteraction)))
      (bind _caninteract (Default|CanInteract _asbp_interaction_station_base self))
      (if _caninteract
        (Variables|Interaction|SetIsInteracting true)
        (bind _output_get (Variables|Interaction|SetInteractingStation _asbp_interaction_station_base))
        (Default|StartInteracting _output_get self)))))

(fn StopInteracting
  (Utilities|IsValid (Variables|Interaction|GetInteractingStation)
    (:Is%20Valid
      (Variables|Interaction|SetIsInteracting false)
      (Default|StopInteracting (Variables|Interaction|GetInteractingStation))
      (Variables|Interaction|SetInteractingStation 0))))

(fn AddIdentityTime
  (params (Time :type Float%20%28double-precision%29))
  (Variables|Identity|SetCurrentIdentityTime (Math|Float|Clamp(Float) (+ Time (Variables|Identity|GetCurrentIdentityTime)) 0.0 (Variables|Identity|GetIdentityMaxTime))))

(fn UpdateClosestInteraction
  (LocalVariables|SetMyLocation (Transformation|GetActorLocation))
  (LocalVariables|SetClosestDistanceSqr (LocalVariables|GetFLT_MAX))
  (for _array_element (Variables|Interaction|GetInteractingActors)
    (if (<= (Class|KismetMathLibrary|VectorDistanceSquared (Transformation|GetActorLocation _array_element) (LocalVariables|GetMyLocation)) (LocalVariables|GetClosestDistanceSqr))
      (LocalVariables|SetClosestDistanceSqr (Class|KismetMathLibrary|VectorDistanceSquared (Transformation|GetActorLocation _array_element) (LocalVariables|GetMyLocation)))
      (LocalVariables|SetClosestActor _array_element)))
  (Variables|Interaction|SetClosestInteraction (LocalVariables|GetClosestActor)))

(fn UpdateAnimation
  (bind _animinstance (Variables|Components|GetAnimInstance))
  (Utilities|IsValid _animinstance
    (:Is%20Valid
      (Variables|/Game/Characters/Mannequins/Anims/Unarmed/ABP_Unarmed.ABP_Unarmed_C|SetIsInteracting _animinstance (Variables|Interaction|GetIsInteracting)))))

(fn UpdateUITimer
  (bind _ui_bitmask_identity (Variables|Default|GetUI%20Bitmask%20Identity))
  (Utilities|IsValid _ui_bitmask_identity
    (:Is%20Valid
      (Variables|/Game/UI/UI_BitmaskIdentity.UI_BitmaskIdentity_C|SetIdentityTimerRemaining _ui_bitmask_identity (/ (Variables|Identity|GetCurrentIdentityTime) (Variables|Identity|GetIdentityMaxTime))))))

(fn PerformArrest
  (Variables|Default|SetIsArrested true)
  (Interaction|StopInteracting)
  (CallFunction|StopSampling)
  (Input|DisableInput (Game|GetPlayerController 0)))

(fn CompleteSampling
  (params (Identity :type EIdentityType%20Enum :default "NewEnumerator0"))
  (bind _ui_bitmask_identity (Variables|Default|GetUI%20Bitmask%20Identity))
  (Identity|UpdateIdentity Identity)
  (Utilities|FlowControl|Sequence
    (:then_0
      (Utilities|IsValid _ui_bitmask_identity
        (:Is%20Valid
          (Variables|/Game/UI/UI_BitmaskIdentity.UI_BitmaskIdentity_C|SetIsSampling _ui_bitmask_identity false)
          (Variables|/Game/UI/UI_BitmaskIdentity.UI_BitmaskIdentity_C|SetSamplingTime _ui_bitmask_identity 0.0)
          (Variables|/Game/UI/UI_BitmaskIdentity.UI_BitmaskIdentity_C|SetIdentityTimerRemaining _ui_bitmask_identity 1.0))))
    (:then_1
      (Variables|Identity|SetCurrentIdentityTime (Variables|Identity|GetIdentityMaxTime))
      (Variables|Sampling|SetIsSampling false)
      (Variables|Sampling|SetCurrentSamplingTime 0.0)
      (Variables|Sampling|SetSamplingNPC 0)
      (return))))