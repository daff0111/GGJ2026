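; BP_WorkerStation is an interactable station that repeatedly adds identity time to the player working at it.
; Its trigger overlap registers and unregisters it as an interacting actor on BP_PlayerCharacter.
; Tick swaps component visibility while the station is active or reserved.
; During interaction, Tick grants time and resets the timer whenever the threshold is reached, or stops the player if CanInteract fails.
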(event OnComponentBeginOverlap(InteractionTrigger)
  (params (OverlappedComponent :type Primitive%20Component%20Object%20Reference) (OtherActor :type Actor%20Object%20Reference) (OtherComp :type Primitive%20Component%20Object%20Reference) (OtherBodyIndex :type Integer) (bFromSweep :type Boolean) (SweepResult :type Hit%20Result%20Structure%20%28by%20ref%29))
  (bind _asbp_player_character (Utilities|Casting|CastToBP_PlayerCharacter OtherActor))
  (Default|AddInteractingActor _asbp_player_character self))

(event OnComponentEndOverlap(InteractionTrigger)
  (params (OverlappedComponent :type Primitive%20Component%20Object%20Reference) (OtherActor :type Actor%20Object%20Reference) (OtherComp :type Primitive%20Component%20Object%20Reference) (OtherBodyIndex :type Integer))
  (bind _asbp_player_character (Utilities|Casting|CastToBP_PlayerCharacter OtherActor))
  (Default|RemoveInteractingActor _asbp_player_character self))

(event EventTick
  (params (DeltaSeconds :type Float%20%28single-precision%29))
  (bind _interactingplayer (Variables|Default|GetInteractingPlayer))
  (bind _interactionactive (Variables|Default|GetInteractionActive))
  (bind _is_reserved (Variables|Default|GetIs%20Reserved))
  (bind _returnvalue (or _interactionactive _is_reserved))
  (|CallParentFunction DeltaSeconds)
  (Rendering|SetVisibility (Variables|Default|GetMesh3) _returnvalue false)
  (Rendering|SetVisibility (not _returnvalue) false)
  (if (Variables|Default|GetInteractionActive)
    (bind _caninteract (CallFunction|CanInteract _interactingplayer))
    (if _caninteract
      (if (>= (Variables|Default|GetCurrentInteractionTime) (Variables|Default|GetInteractionThreshold))
        (Default|AddIdentityTime (Variables|Default|GetInteractingPlayer) (Variables|Default|GetIndentityTimeAdded))
        (Variables|Default|SetCurrentInteractionTime 0.0))
      (else
        (Default|StopInteracting _interactingplayer)))))

(fn ConstructionScript)