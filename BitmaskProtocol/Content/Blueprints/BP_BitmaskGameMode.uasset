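; BP_BitmaskGameMode is the game mode for a simple game, tracking score, NPC population cap and a global guard alert level.
; Raising the alert level alerts security NPCs near the last known player location, with radius and guard-count limit scaling by level.
; Scoring uses a combo multiplier that builds with score events and decays through a retriggerable cooldown.
; It drives the UI widget directly, though the widget creation nodes are unwired.
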(event Custom|ComboManager
  ;[0.15 0.15 0.15 0.502] Scoring System - uses a simple combo multiplier with cooldown.
  (Utilities|FlowControl|Sequence
    (:then_0
      (bind _result (Math|Integer|IncrementInt (Variables|Scoring|GetComboIncrement))
        (:%20%20
          (if (and (> _result (Variables|Scoring|GetComboIncrementMax)) (<= (Variables|Scoring|GetCombo) (Variables|Scoring|GetComboCap)))
            (bind _result_2 (Math|Integer|IncrementInt (Variables|Scoring|GetCombo))
              (:%20%20
                (Default|ComboUpdate (Variables|UserInterface|GetUI%20Widget) _result_2)
                (Variables|Scoring|SetComboIncrement 0)))))))
    (:then_1
      (Utilities|FlowControl|RetriggerableDelay (Variables|Scoring|GetComboCooldown))
      (if (> (Variables|Scoring|GetCombo) 1)
        (bind _result_3 (Math|Integer|DecrementInt (Variables|Scoring|GetCombo))
          (:%20%20
            (Default|ComboUpdate (Variables|UserInterface|GetUI%20Widget) _result_3)
            (Variables|Scoring|SetComboIncrement 0)
            (CallFunction|ComboTimer)))))))

(event Custom|Decrease%20NPCs
  ;[0.15 0.15 0.15 0.5] Manage NPC counts on the level
  (Math|Integer|DecrementInt (Variables|NPCs|GetCurrent%20NPC%20Count)))

(event Custom|ComboTimer
  ;[0.15 0.15 0.15 0.502] Scoring System - uses a simple combo multiplier with cooldown.
  (Utilities|FlowControl|RetriggerableDelay (Variables|Scoring|GetComboCooldown))
  (if (> (Variables|Scoring|GetCombo) 1)
    (bind _result (Math|Integer|DecrementInt (Variables|Scoring|GetCombo))
      (:%20%20
        (Default|ComboUpdate (Variables|UserInterface|GetUI%20Widget) _result)
        (Variables|Scoring|SetComboIncrement 0)
        (CallFunction|ComboTimer)))))

(event Custom|Increase%20NPCs
  ;[0.15 0.15 0.15 0.5] Manage NPC counts on the level
  (Math|Integer|IncrementInt (Variables|NPCs|GetCurrent%20NPC%20Count)))

(event Custom|RaiseAlertLevel
  (params (AlertLevel :type Integer))
  (Variables|Default|SetGlobalAlertLevel (Math|Integer|Min(Integer) (Math|Integer|Max(Integer) AlertLevel (Variables|Default|GetGlobalAlertLevel)) (Variables|Default|GetMaxAlertLevel)))
  (CallFunction|AlertGuardsinDistance))

(event EventBeginPlay
  ;[0.15 0.15 0.15 0.502] As this is a very simple game, we're managing the UI from the Game Mode rather than a dedicated HUD actor
  (bind _outactors (Actor|GetAllActorsOfClass "/Game/Blueprints/BP_NPC_Security.BP_NPC_Security_C"))
  (Variables|Default|SetSecurityNPCs _outactors))

(event EventScoreUpdate
  (params (NewValue :type Integer))
  ;[0.15 0.15 0.15 0.502] Scoring System - uses a simple combo multiplier with cooldown.
  (bind _output_get (Variables|Scoring|SetScore (+ (Variables|Scoring|GetScore) (* (Variables|Scoring|GetCombo) NewValue))))
  (Default|ScoreUpdate (Variables|UserInterface|GetUI%20Widget) _output_get)
  (CallFunction|ComboManager))

(event EventTick
  (params (DeltaSeconds :type Float%20%28single-precision%29))
  (bind _lastplayerlocation (Variables|Default|GetLastPlayerLocation))
  (if (Utilities|Operators|NotEqual(!=) :A _lastplayerlocation)
    (Rendering|Debug|DrawDebugSphere _lastplayerlocation 5e+01 12 "(R=0.916060,G=1.000000,B=0.044922,A=1.000000)" 0.0 1.0)))

(fn ConstructionScript)

(fn ShouldSpawnNPCs
  (return (<= (Variables|NPCs|GetCurrent%20NPC%20Count) (Variables|NPCs|GetMax%20NPC%20Cap))))

(fn SetLastPlayerLocation
  (params (LastPlayerLocation :type Vector))
  (Variables|Default|SetLastPlayerLocation LastPlayerLocation))

(fn AlertGuardsinDistance
  (LocalVariables|SetAlertDistance (* (Variables|Default|GetAlert%20DistancePerLevel) (Variables|Default|GetGlobalAlertLevel)))
  (bind _array_element (Utilities|Array|ForEachLoopwithBreak (Variables|Default|GetSecurityNPCs) :!label _label)
    (:LoopBody
      (if (or (Utilities|Enum|Equal(Enum) (Variables|/Game/Blueprints/BP_NPC_Base.BP_NPC_Base_C|GetAlertLevel _array_element) "NewEnumerator0") (Utilities|Enum|Equal(Enum) (Variables|/Game/Blueprints/BP_NPC_Base.BP_NPC_Base_C|GetAlertLevel _array_element) "NewEnumerator1"))
        (if (<= (Math|Vector|Distance2D(Vector) (Variables|Default|GetLastPlayerLocation) (Transformation|GetActorLocation _array_element)) (LocalVariables|GetAlertDistance))
          (Variables|/Game/Blueprints/BP_NPC_Base.BP_NPC_Base_C|SetAlertLevel _array_element "NewEnumerator2")
          (bind _result (Math|Integer|IncrementInt (LocalVariables|GetAlertGuards))
            (:%20%20
              (bind _output_get (LocalVariables|SetAlertGuards _result))
              (if (>= _output_get (Variables|Default|GetGlobalAlertLevel))
                (goto _label Break)))))))))