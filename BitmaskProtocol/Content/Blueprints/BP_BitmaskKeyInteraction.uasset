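; Key pickup interaction station that the player collects by holding an interaction until a time threshold is reached.
; Trigger overlaps register it with the player, while Tick swaps active and idle meshes, cancels invalid interactions and fires GetKey once on completion.
; GetKey locks the station, hides a mesh, gives the player the key and unlocks every switch-and-door station.
; It also notifies the game mode, raising the alert level and recording player location and identity.
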(event OnComponentBeginOverlap(InteractionTrigger)
  (params (OverlappedComponent :type Primitive%20Component%20Object%20Reference) (OtherActor :type Actor%20Object%20Reference) (OtherComp :type Primitive%20Component%20Object%20Reference) (OtherBodyIndex :type Integer) (bFromSweep :type Boolean) (SweepResult :type Hit%20Result%20Structure%20%28by%20ref%29))
  (bind _asbp_player_character (Utilities|Casting|CastToBP_PlayerCharacter OtherActor))
  (Default|AddInteractingActor _asbp_player_character self))

(event OnComponentEndOverlap(InteractionTrigger)
  (params (OverlappedComponent :type Primitive%20Component%20Object%20Reference) (OtherActor :type Actor%20Object%20Reference) (OtherComp :type Primitive%20Component%20Object%20Reference) (OtherBodyIndex :type Integer))
  (bind _asbp_player_character (Utilities|Casting|CastToBP_PlayerCharacter OtherActor))
  (Default|RemoveInteractingActor _asbp_player_character self))

(event Custom|GetKey
  (bind _interactingplayer (Variables|Default|GetInteractingPlayer))
  (Variables|Default|SetLocked true)
  (Rendering|SetVisibility (Variables|Default|GetMesh1) false false)
  (bind _asbp_bitmask_game_mode (Utilities|Casting|CastToBP_BitmaskGameMode (Game|GetGameMode)))
  (Default|GetKey _asbp_bitmask_game_mode)
  (Default|RaiseAlertLevel _asbp_bitmask_game_mode 3)
  (Default|SetLastPlayerLocation _asbp_bitmask_game_mode (Transformation|GetActorLocation _interactingplayer))
  (Default|SetLastPlayerIdentity _asbp_bitmask_game_mode (Variables|/Game/Blueprints/BP_PlayerCharacter.BP_PlayerCharacter_C|GetCurrentIdentity _interactingplayer))
  (Variables|/Game/Blueprints/BP_PlayerCharacter.BP_PlayerCharacter_C|SetHasKey _interactingplayer true)
  (bind _outactors (Actor|GetAllActorsOfClass "/Game/Blueprints/BP_InteractionStationSwitchAndDoor.BP_InteractionStationSwitchAndDoor_C"))
  (for _array_element _outactors
    (Default|Unlock _array_element)))

(event EventTick
  (params (DeltaSeconds :type Float%20%28single-precision%29))
  (bind _interactingplayer (Variables|Default|GetInteractingPlayer))
  (bind _interactionactive (Variables|Default|GetInteractionActive))
  (|CallParentFunction DeltaSeconds)
  (Rendering|SetVisibility (Variables|Default|GetMesh2) (not _interactionactive) false)
  (Rendering|SetVisibility (Variables|Default|GetMesh3) _interactionactive false)
  (if (Variables|Default|GetInteractionActive)
    (bind _caninteract (CallFunction|CanInteract _interactingplayer))
    (if _caninteract
      (if (>= (Variables|Default|GetCurrentInteractionTime) (Variables|Default|GetInteractionThreshold))
        (Utilities|FlowControl|DoOnce false
          (:Completed
            (CallFunction|GetKey))))
      (else
        (Default|StopInteracting _interactingplayer)))))

(fn ConstructionScript)

(fn CanInteract
  (params (Character :type BP%20Player%20Character%20Object%20Reference))
  (bind _caninteract (|CallParentFunction Character))
  (return (and _caninteract (not (Variables|Default|GetLocked)))))