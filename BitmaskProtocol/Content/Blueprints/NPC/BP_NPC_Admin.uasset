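; Admin NPC Blueprint that overrides UpdateSuspicion to judge the perceived player by mask identity and behavior.
; Trespassing and some identities raise suspicion at full rate, while worker or security disguises raise it slower when not interacting or off the security path.
; Full suspicion turns the NPC Aggressive and reports alert, player location and identity to the game mode; otherwise it drains back to Calm.
; When Searching or Aggressive, suspicious sightings trigger Aggressive immediately, otherwise Searching.
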(event EventBeginPlay
  (|CallParentFunction) ; This node is disabled and will not be called.\nDrag off pins to build functionality.
)

(event Collision|EventActorBeginOverlap
  (params (OtherActor :type Actor%20Object%20Reference)))

(event EventTick
  (params (DeltaSeconds :type Float%20%28single-precision%29))
  (|CallParentFunction DeltaSeconds) ; This node is disabled and will not be called.\nDrag off pins to build functionality.
)

(fn ConstructionScript
  (|CallParentFunction))

(fn UpdateSuspicion
  (params (DeltaTime :type Float%20%28double-precision%29))
  (bind _suspicionraiserate (Variables|Default|GetSuspicionRaiseRate))
  (bind _perceivedplayer (Variables|Default|GetPerceivedPlayer))
  (bind _bitmask_game_mode (Variables|Default|GetBitmask%20Game%20Mode))
  (bind _maxlocalsuspicion (Variables|Default|GetMaxLocalSuspicion))
  (bind _perceivedplayer_2 (Variables|Default|GetPerceivedPlayer))
  (bind _istrespassing (Variables|/Game/Blueprints/BP_PlayerCharacter.BP_PlayerCharacter_C|GetIsTrespassing _perceivedplayer))
  (bind _isclosetosecuritypath (Variables|/Game/Blueprints/BP_PlayerCharacter.BP_PlayerCharacter_C|GetIsCloseToSecurityPath _perceivedplayer))
  (bind _currentidentity (Variables|/Game/Blueprints/BP_PlayerCharacter.BP_PlayerCharacter_C|GetCurrentIdentity _perceivedplayer))
  (bind _isinteracting (Variables|/Game/Blueprints/BP_PlayerCharacter.BP_PlayerCharacter_C|GetIsInteracting _perceivedplayer))
  (bind _returnvalue (not _isinteracting))
  (bind _returnvalue_2 (not _isclosetosecuritypath))
  (bind _returnvalue_3 (Utilities|Enum|Equal(Enum) _currentidentity "NewEnumerator0"))
  (bind _returnvalue_4 (Utilities|Enum|Equal(Enum) _currentidentity "NewEnumerator2"))
  (bind _returnvalue_5 (Utilities|Enum|Equal(Enum) _currentidentity "NewEnumerator4"))
  (bind _returnvalue_6 (Utilities|Enum|Equal(Enum) _currentidentity "NewEnumerator1"))
  (bind _returnvalue_7 (and _returnvalue_6 _returnvalue))
  (bind _returnvalue_8 (and _returnvalue_4 _returnvalue_2))
  (bind _returnvalue_9 (Math|Boolean|ORBoolean _returnvalue_3 _istrespassing _returnvalue_5))
  (bind _returnvalue_10 (Math|Boolean|ORBoolean _returnvalue_9 _returnvalue_7 _returnvalue_8 _returnvalue_5))
  (|CallParentFunction DeltaTime)
  (switch Utilities|FlowControl|Switch|SwitchonEAlertState (Variables|Default|GetAlertLevel)
    (:NewEnumerator0
      (Utilities|IsValid (Variables|Default|GetPerceivedPlayer) :!label _label
        (:Is%20Valid
          (if _returnvalue_10
            (LocalVariables|SetSuspicionRaiseRateLocal (select _returnvalue_9 _suspicionraiserate (* _suspicionraiserate 0.4)))
            (if (Utilities|Enum|Equal(Enum) (Variables|Default|GetAlertLevel) "NewEnumerator0")
              (CallFunction|SetAlertedState "NewEnumerator1"))
            (bind _output_get (Variables|Default|SetLocalSuspicion (Math|Float|Min(Float) (+ (Variables|Default|GetLocalSuspicion) (* DeltaTime (LocalVariables|GetSuspicionRaiseRateLocal))) _maxlocalsuspicion)))
            (if (>= _output_get _maxlocalsuspicion)
              (Default|RaiseAlertLevel (Variables|Default|GetBitmask%20Game%20Mode) 5)
              (CallFunction|SetAlertedState "NewEnumerator3")
              (Default|SetLastPlayerLocation _bitmask_game_mode (Transformation|GetActorLocation _perceivedplayer_2))
              (Default|SetLastPlayerIdentity _bitmask_game_mode (Variables|/Game/Blueprints/BP_PlayerCharacter.BP_PlayerCharacter_C|GetCurrentIdentity _perceivedplayer_2)))
            (else
              (if (> (Variables|Default|GetLocalSuspicion) 0.0) :!label _label_2
                (CallFunction|SetAlertedState "NewEnumerator1")
                (bind _output_get_2 (Variables|Default|SetLocalSuspicion (Math|Float|Max(Float) (- (Variables|Default|GetLocalSuspicion) (* DeltaTime (Variables|Default|GetSuspicionDrainRate))) 0.0)))
                (if (== _output_get_2 0.0)
                  (CallFunction|SetAlertedState "NewEnumerator0"))))))
        (:Is%20Not%20Valid
          (goto _label_2))))
    (:NewEnumerator1
      (goto _label))
    (:NewEnumerator2
      (Utilities|IsValid (Variables|Default|GetPerceivedPlayer) :!label _label_3
        (:Is%20Valid
          (if _returnvalue_10
            (CallFunction|SetAlertedState "NewEnumerator3")
            (else
              (CallFunction|SetAlertedState "NewEnumerator2" :!label _label_4))))
        (:Is%20Not%20Valid
          (goto _label_4))))
    (:NewEnumerator3
      (goto _label_3))))