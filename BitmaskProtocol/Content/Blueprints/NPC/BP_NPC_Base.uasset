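; Base NPC for a stealth game where the player samples identities from characters such as Workers, Security, Supervisors and Admins.
; Identity tints the mesh materials, and an overlap sphere registers the NPC with the player as a sampling target.
; Sight perception tracks non-hiding players, blocks their sampling and reports detections to the game mode when alerted.
; Tick drives animation, debug text and an empty suspicion hook, while interacting turns the NPC into a nav obstacle.
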(event OnComponentBeginOverlap(Sphere)
  (params (OverlappedComponent :type Primitive%20Component%20Object%20Reference) (OtherActor :type Actor%20Object%20Reference) (OtherComp :type Primitive%20Component%20Object%20Reference) (OtherBodyIndex :type Integer) (bFromSweep :type Boolean) (SweepResult :type Hit%20Result%20Structure%20%28by%20ref%29))
  ;[0.15 0.15 0.15 0.5] Sampling
  (bind _asbp_player_character (Utilities|Casting|CastToBP_PlayerCharacter OtherActor))
  (Default|AddSamplingActor _asbp_player_character self))

(event OnComponentEndOverlap(Sphere)
  (params (OverlappedComponent :type Primitive%20Component%20Object%20Reference) (OtherActor :type Actor%20Object%20Reference) (OtherComp :type Primitive%20Component%20Object%20Reference) (OtherBodyIndex :type Integer))
  ;[0.15 0.15 0.15 0.5] Sampling
  (bind _asbp_player_character (Utilities|Casting|CastToBP_PlayerCharacter OtherActor))
  (Default|RemoveSamplingActor _asbp_player_character self))

(event EventTick
  (params (DeltaSeconds :type Float%20%28single-precision%29))
  ;[0.15 0.15 0.15 0.5] Tick
  (Utilities|FlowControl|Sequence
    (:then_0
      (CallFunction|UpdateAnimation))
    (:then_1
      (CallFunction|UpdateSuspicion DeltaSeconds))
    (:then_2
      (CallFunction|UpdateDebugText))))

(event EventBeginPlay
  ;[0.1771 0.6771 0.08265 0.5] Begin Play
  (Utilities|Time|SetTimerbyEvent (EventDispatchers|CreateEvent :!event UpdateAIPlayerPerception) 0.2 true false 0.15)
  (bind _asbp_bitmask_game_mode (Utilities|Casting|CastToBP_BitmaskGameMode (Game|GetGameMode)))
  (Variables|NPC|SetBitmask%20Game%20Mode _asbp_bitmask_game_mode)
  (bind _asabp_unarmed (Utilities|Casting|CastToABP_Unarmed (Components|SkeletalMesh|GetAnimInstance (Variables|Character|GetMesh))))
  (bind _output_get (Variables|NPC|SetAnimInstance _asabp_unarmed))
  (Variables|/Game/Characters/Mannequins/Anims/Unarmed/ABP_Unarmed.ABP_Unarmed_C|SetIsAI _output_get true)
  (Class|NavRelevantComponent|SetNavigationRelevancy (Variables|Default|GetNavModifier) false))

(event EventCompleteSampling
  (params (Identity :type EIdentityType%20Enum :default "NewEnumerator0"))
  ;[0.15 0.15 0.15 0.5] Sampling
)

(event EventStartSampling
  (params (Requester :type Actor%20Object%20Reference))
  ;[0.15 0.15 0.15 0.5] Sampling
)

(fn ConstructionScript
  (bind _mesh (Variables|Character|GetMesh))
  (bind _mymaterials (Variables|NPC|GetMyMaterials))
  (Utilities|FlowControl|Sequence
    (:then_0
      (bind _returnvalue (Rendering|Material|CreateDynamicMaterialInstance _mesh 0 0 "None" :!class /Script/Engine.PrimitiveComponent))
      (Utilities|Array|Add _mymaterials _returnvalue))
    (:then_1
      (bind _returnvalue_2 (Rendering|Material|CreateDynamicMaterialInstance _mesh 1 0 "None" :!class /Script/Engine.PrimitiveComponent))
      (Utilities|Array|Add _mymaterials _returnvalue_2))
    (:then_2
      (CallFunction|UpdateMaterials (Variables|NPC|GetIdentity)))
    (:then_3
      (Components|Sphere|SetSphereRadius (Variables|Default|GetSphere) (Variables|NPC|GetSamplingRadius) true))))

(fn UpdateMaterials
  (params (CurrentIdentity :type EIdentityType%20Enum :default "NewEnumerator0"))
  (Rendering|Material|SetVectorParameterValue (Variables|NPC|GetMyMaterials) "Paint Tint" (Utilities|Select :Index CurrentIdentity :NewEnumerator0 "(R=1.000000,G=1.000000,B=1.000000,A=1.000000)" :NewEnumerator1 "(R=0.000000,G=0.472568,B=1.000000,A=1.000000)" :NewEnumerator2 "(R=1.000000,G=0.013193,B=0.000000,A=1.000000)" :NewEnumerator3 "(R=1.000000,G=0.885625,B=0.000000,A=1.000000)" :NewEnumerator4 "(R=0.562971,G=0.000000,B=1.000000,A=1.000000)") :!class /Script/Engine.MaterialInstanceDynamic))

(fn CanSample
  (bind _perceivedplayer (Variables|NPC|GetPerceivedPlayer))
  (if (not (Utilities|IsValid _perceivedplayer))
    (return true)
    (else
      (return (Utilities|Enum|Equal(Enum) (Variables|/Game/Blueprints/BP_PlayerCharacter.BP_PlayerCharacter_C|GetCurrentIdentity _perceivedplayer) (Variables|NPC|GetIdentity))))))

(fn UpdateAnimation
  (bind _animinstance (Variables|NPC|GetAnimInstance))
  (Utilities|IsValid (Variables|NPC|GetAnimInstance)
    (:Is%20Valid
      (Utilities|IsValid (Variables|NPC|GetPerceivedPlayer)
        (:Is%20Valid
          (if (> (Variables|Suspicion|GetLocalSuspicion) 0.0)
            (Variables|/Game/Characters/Mannequins/Anims/Unarmed/ABP_Unarmed.ABP_Unarmed_C|SetIsSuspicious _animinstance true)
            (Variables|/Game/Characters/Mannequins/Anims/Unarmed/ABP_Unarmed.ABP_Unarmed_C|SetLookAtRotation _animinstance (Math|Rotator|MakeRotator 0.0 0.0 (- (.yaw (Math|Rotator|FindLookatRotation (Transformation|GetActorLocation) (Transformation|GetActorLocation (Variables|NPC|GetPerceivedPlayer)))) (.yaw (Transformation|GetActorRotation)))))
            (else
              (Variables|/Game/Characters/Mannequins/Anims/Unarmed/ABP_Unarmed.ABP_Unarmed_C|SetIsSuspicious _animinstance false :!label _label))))
        (:Is%20Not%20Valid
          (goto _label))))))

(fn SetIsInteracting
  (params (IsInteracting :type Boolean))
  (bind _navmodifier (Variables|Default|GetNavModifier))
  (bind _output_get (Variables|NPC|SetIs%20Interacting IsInteracting))
  (bind _output_get_2 (Variables|/Game/Characters/Mannequins/Anims/Unarmed/ABP_Unarmed.ABP_Unarmed_C|SetIsInteracting (Variables|NPC|GetAnimInstance) _output_get))
  (Class|NavModifierComponent|SetAreaClass _navmodifier (select _output_get_2 "/Script/NavigationSystem.NavArea_Obstacle" "/Script/NavigationSystem.NavArea_Default"))
  (Class|NavRelevantComponent|SetNavigationRelevancy _navmodifier _output_get_2))

(fn UpdateDebugText
  (bind _textrender (Variables|Default|GetTextRender))
  (bind _aggressive (LocalVariables|GetAggressive))
  (Rendering|Components|TextRender|SetText _textrender (Utilities|Text|ToText(Integer) (Math|Float|Truncate (Variables|Suspicion|GetLocalSuspicion))))
  (Rendering|Components|TextRender|SetTextRenderColor _textrender (Utilities|Select :Index (Variables|NPC|GetAlertLevel) :NewEnumerator0 (LocalVariables|GetCalm) :NewEnumerator1 (LocalVariables|GetAlert) :NewEnumerator2 (LocalVariables|GetSearching) :NewEnumerator3 _aggressive :NewEnumerator4 _aggressive)))

(fn IsPlayerDetected
  (params (PlayerCharacter :type BP%20Player%20Character%20Object%20Reference))
  (bind _currentidentity (Variables|/Game/Blueprints/BP_PlayerCharacter.BP_PlayerCharacter_C|GetCurrentIdentity PlayerCharacter))
  (return (Math|Boolean|ANDBoolean (Utilities|Enum|NotEqual(Enum) (Variables|NPC|GetAlertLevel) "NewEnumerator0") (or (Utilities|Enum|Equal(Enum) (Variables|/Game/Blueprints/BP_BitmaskGameMode.BP_BitmaskGameMode_C|GetLastPlayerIdentity (Variables|NPC|GetBitmask%20Game%20Mode)) _currentidentity) (Utilities|Enum|Equal(Enum) _currentidentity "NewEnumerator0")) (not (Variables|/Game/Blueprints/BP_PlayerCharacter.BP_PlayerCharacter_C|GetIsHiding PlayerCharacter)))))

(fn UpdateAIPlayerPerception
  (bind _bitmask_game_mode (Variables|NPC|GetBitmask%20Game%20Mode))
  (bind _aiperception (Variables|Default|GetAIPerception))
  (bind _outactors (Class|AIPerceptionComponent|GetCurrentlyPerceivedActors _aiperception "/Script/AIModule.AISense_Sight"))
  (if (> (Utilities|Array|Length _outactors) 0)
    (bind _asbp_player_character (Utilities|Casting|CastToBP_PlayerCharacter (Utilities|Array|Get(acopy) _outactors))
      (:then
        (if (Variables|/Game/Blueprints/BP_PlayerCharacter.BP_PlayerCharacter_C|GetIsHiding _asbp_player_character)
          (Utilities|IsValid (Variables|NPC|GetPerceivedPlayer) :!label _label
            (:Is%20Valid
              (Variables|/Game/Blueprints/BP_PlayerCharacter.BP_PlayerCharacter_C|SetCanSample (Variables|NPC|GetPerceivedPlayer) true)
              (Variables|NPC|SetPerceivedPlayer 0)))
          (else
            (bind _output_get (Variables|NPC|SetPerceivedPlayer _asbp_player_character))
            (Variables|/Game/Blueprints/BP_PlayerCharacter.BP_PlayerCharacter_C|SetCanSample _output_get false)
            (if (CallFunction|IsPlayerDetected _output_get)
              (Default|SetLastPlayerLocation _bitmask_game_mode (Transformation|GetActorLocation _output_get))
              (Default|SetLastPlayerIdentity _bitmask_game_mode (Variables|/Game/Blueprints/BP_PlayerCharacter.BP_PlayerCharacter_C|GetCurrentIdentity _output_get))))))
      (:CastFailed
        (goto _label)))
    (else
      (goto _label))))

(fn UpdateSuspicion
  (params (DeltaTime :type Float%20%28double-precision%29)))

(fn SetAlertedState
  (params (AlertLevel :type EAlertState%20Enum :default "NewEnumerator0"))
  (if (Utilities|Enum|NotEqual(Enum) AlertLevel (Variables|NPC|GetAlertLevel))
    (Variables|NPC|SetAlertLevel AlertLevel)))