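; Supervisor NPC that builds suspicion of a perceived player based on their mask identity and behavior, overriding the parent's UpdateSuspicion.
; Trespassing or one identity raises suspicion at full rate, another at half rate while not interacting, and a third only when trespassing.
; At maximum it raises the game mode's alert level and records the player's location and identity.
; Otherwise suspicion drains, returning the NPC to its base alert state at zero.
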(event EventBeginPlay
  (|CallParentFunction) ; This node is disabled and will not be called.\nDrag off pins to build functionality.
)

(event Collision|EventActorBeginOverlap
  (params (OtherActor :type Actor%20Object%20Reference)))

(event EventTick
  (params (DeltaSeconds :type Float%20%28single-precision%29))
  (|CallParentFunction DeltaSeconds) ; This node is disabled and will not be called.\nDrag off pins to build functionality.
)

(fn ConstructionScript
  (|CallParentFunction))

(fn UpdateSuspicion
  (params (DeltaTime :type Float%20%28double-precision%29))
  (bind _perceivedplayer (Variables|Default|GetPerceivedPlayer))
  (bind _suspicionraiserate (Variables|Default|GetSuspicionRaiseRate))
  (bind _bitmask_game_mode (Variables|Default|GetBitmask%20Game%20Mode))
  (bind _maxlocalsuspicion (Variables|Default|GetMaxLocalSuspicion))
  (bind _perceivedplayer_2 (Variables|Default|GetPerceivedPlayer))
  (bind _istrespassing (Variables|/Game/Blueprints/BP_PlayerCharacter.BP_PlayerCharacter_C|GetIsTrespassing _perceivedplayer))
  (bind _currentidentity (Variables|/Game/Blueprints/BP_PlayerCharacter.BP_PlayerCharacter_C|GetCurrentIdentity _perceivedplayer))
  (bind _returnvalue (Utilities|Enum|Equal(Enum) _currentidentity "NewEnumerator0"))
  (bind _returnvalue_2 (or _returnvalue _istrespassing))
  (|CallParentFunction DeltaTime)
  (Utilities|IsValid (Variables|Default|GetPerceivedPlayer)
    (:Is%20Valid
      (if (Math|Boolean|ORBoolean _returnvalue_2 (and (Utilities|Enum|Equal(Enum) _currentidentity "NewEnumerator1") (not (Variables|/Game/Blueprints/BP_PlayerCharacter.BP_PlayerCharacter_C|GetIsInteracting _perceivedplayer))) (and (Utilities|Enum|Equal(Enum) _currentidentity "NewEnumerator2") false))
        (LocalVariables|SetSuspicionRaiseRateLocal (select _returnvalue_2 _suspicionraiserate (* _suspicionraiserate 0.5)))
        (if (Utilities|Enum|Equal(Enum) (Variables|Default|GetAlertLevel) "NewEnumerator0")
          (Variables|Default|SetAlertLevel "NewEnumerator1"))
        (bind _output_get (Variables|Default|SetLocalSuspicion (Math|Float|Min(Float) (+ (Variables|Default|GetLocalSuspicion) (* DeltaTime (LocalVariables|GetSuspicionRaiseRateLocal))) _maxlocalsuspicion)))
        (if (>= _output_get _maxlocalsuspicion)
          (Default|RaiseAlertLevel (Variables|Default|GetBitmask%20Game%20Mode) 3)
          (Variables|Default|SetAlertLevel "NewEnumerator3")
          (Default|SetLastPlayerLocation _bitmask_game_mode (Transformation|GetActorLocation _perceivedplayer_2))
          (Default|SetLastPlayerIdentity _bitmask_game_mode (Variables|/Game/Blueprints/BP_PlayerCharacter.BP_PlayerCharacter_C|GetCurrentIdentity _perceivedplayer_2)))
        (else
          (if (> (Variables|Default|GetLocalSuspicion) 0.0) :!label _label
            (Variables|Default|SetAlertLevel "NewEnumerator1")
            (bind _output_get_2 (Variables|Default|SetLocalSuspicion (Math|Float|Max(Float) (- (Variables|Default|GetLocalSuspicion) (* DeltaTime (Variables|Default|GetSuspicionDrainRate))) 0.0)))
            (if (== _output_get_2 0.0)
              (Variables|Default|SetAlertLevel "NewEnumerator0"))))))
    (:Is%20Not%20Valid
      (goto _label))))