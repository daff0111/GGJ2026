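; Worker NPC that builds suspicion of a perceived player and can raise the game's alert level.
; Its UpdateSuspicion override extends the parent's, raising local suspicion over time while the player holds one specific identity and draining it otherwise.
; Reaching maximum suspicion from the base alert state advances the NPC's alert level and notifies BitmaskGameMode; draining to zero resets only the NPC's own level.
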(fn ConstructionScript
  (|CallParentFunction))

(fn UpdateSuspicion
  (params (DeltaTime :type Float%20%28double-precision%29))
  (bind _maxlocalsuspicion (Variables|Default|GetMaxLocalSuspicion))
  (bind _perceivedplayer (Variables|Default|GetPerceivedPlayer))
  (|CallParentFunction DeltaTime)
  (Utilities|IsValid _perceivedplayer
    (:Is%20Valid
      (if (Utilities|Enum|Equal(Enum) (Variables|/Game/Blueprints/BP_PlayerCharacter.BP_PlayerCharacter_C|GetCurrentIdentity _perceivedplayer) "NewEnumerator0")
        (bind _output_get (Variables|Default|SetLocalSuspicion (Math|Float|Min(Float) (+ (Variables|Default|GetLocalSuspicion) (* DeltaTime (Variables|Default|GetSuspicionRaiseRate))) _maxlocalsuspicion)))
        (if (and (>= _output_get _maxlocalsuspicion) (Utilities|Enum|Equal(Enum) (Variables|Default|GetAlertLevel) "NewEnumerator0"))
          (Variables|Default|SetAlertLevel "NewEnumerator1")
          (Default|RaiseAlertLevel (Variables|Default|GetBitmask%20Game%20Mode) 1))
        (else
          (if (> (Variables|Default|GetLocalSuspicion) 0.0) :!label _label
            (bind _output_get_2 (Variables|Default|SetLocalSuspicion (Math|Float|Max(Float) (- (Variables|Default|GetLocalSuspicion) (* DeltaTime (Variables|Default|GetSuspicionDrainRate))) 0.0)))
            (if (== _output_get_2 0.0)
              (Variables|Default|SetAlertLevel "NewEnumerator0"))))))
    (:Is%20Not%20Valid
      (goto _label))))