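; Security guard NPC that detects the player, escalates through alert states and arrests them on capture-capsule contact while Aggressive.
; Suspicion builds while the perceived player has a particular identity or is trespassing and drains otherwise; maxing out reports location and identity to BitmaskGameMode, raising its alert level.
; Alert or Searching guards turn Aggressive on trespass or the last reported identity, reverting to Searching upon losing the player.
; State changes set walk speed.
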(event OnComponentBeginOverlap(CaptureCapsule)
  (params (OverlappedComponent :type Primitive%20Component%20Object%20Reference) (OtherActor :type Actor%20Object%20Reference) (OtherComp :type Primitive%20Component%20Object%20Reference) (OtherBodyIndex :type Integer) (bFromSweep :type Boolean) (SweepResult :type Hit%20Result%20Structure%20%28by%20ref%29))
  ;[0.15 0.01715 0.007114 0.5] Arrest Player
  (if (Utilities|Enum|Equal(Enum) (Variables|Default|GetAlertLevel) "NewEnumerator3")
    (if (== OtherActor (Variables|Default|GetPerceivedPlayer))
      (CallFunction|Arrest))))

(event Custom|Arrest
  ;[0.15 0.01715 0.007114 0.5] Arrest Player
  (Utilities|FlowControl|DoOnce false
    (:Completed
      (Default|Arrested (Variables|Default|GetPerceivedPlayer))
      (Animation|Montage|MontagePlay (Variables|Default|GetAnimInstance) "/Game/Characters/Mannequins/Anims/Rifle/MF_Rifle_Idle_ADS_Montage.MF_Rifle_Idle_ADS_Montage" 0.0 "MontageLength" 0.0 true)
      (CallFunction|SetAlertedState "NewEnumerator4"))))

(event EventBeginPlay)

(event Collision|EventActorBeginOverlap
  (params (OtherActor :type Actor%20Object%20Reference)))

(fn ConstructionScript
  (|CallParentFunction))

(fn UpdateSuspicion
  (params (DeltaTime :type Float%20%28double-precision%29))
  (bind _bitmask_game_mode (Variables|Default|GetBitmask%20Game%20Mode))
  (bind _maxlocalsuspicion (Variables|Default|GetMaxLocalSuspicion))
  (bind _perceivedplayer (Variables|Default|GetPerceivedPlayer))
  (bind _perceivedplayer_2 (Variables|Default|GetPerceivedPlayer))
  (bind _perceivedplayer_3 (Variables|Default|GetPerceivedPlayer))
  (bind _returnvalue (Utilities|IsValid _perceivedplayer_3))
  (bind _currentidentity (Variables|/Game/Blueprints/BP_PlayerCharacter.BP_PlayerCharacter_C|GetCurrentIdentity _perceivedplayer))
  (bind _returnvalue_2 (Utilities|Enum|Equal(Enum) _currentidentity "NewEnumerator0"))
  (|CallParentFunction DeltaTime)
  (if (not (Utilities|Enum|Equal(Enum) (Variables|Default|GetAlertLevel) "NewEnumerator4"))
    (Utilities|FlowControl|Sequence
      (:then_0
        (switch Utilities|FlowControl|Switch|SwitchonEAlertState (Variables|Default|GetAlertLevel)
          (:NewEnumerator0
            _)
          (:NewEnumerator1
            _))
        (Utilities|IsValid _perceivedplayer
          (:Is%20Valid
            (if (or _returnvalue_2 (Variables|/Game/Blueprints/BP_PlayerCharacter.BP_PlayerCharacter_C|GetIsTrespassing _perceivedplayer))
              (bind _output_get (Variables|Default|SetLocalSuspicion (Math|Float|Min(Float) (+ (Variables|Default|GetLocalSuspicion) (* DeltaTime (Variables|Default|GetSuspicionRaiseRate))) _maxlocalsuspicion)))
              (if (>= _output_get _maxlocalsuspicion)
                (if _returnvalue_2
                  _
                  (else
                    (Variables|/Game/Blueprints/BP_PlayerCharacter.BP_PlayerCharacter_C|SetCurrentIdentityTime (Variables|Default|GetPerceivedPlayer) 0.1)))
                (CallFunction|SetAlertedState "NewEnumerator1")
                (Default|SetLastPlayerLocation _bitmask_game_mode (Transformation|GetActorLocation _perceivedplayer_2))
                (Variables|/Game/Blueprints/BP_BitmaskGameMode.BP_BitmaskGameMode_C|SetLastPlayerIdentity _bitmask_game_mode (Variables|/Game/Blueprints/BP_PlayerCharacter.BP_PlayerCharacter_C|GetCurrentIdentity _perceivedplayer_2))
                (Default|RaiseAlertLevel _bitmask_game_mode 2))
              (else
                (bind _output_get_2 (Variables|Default|SetLocalSuspicion (Math|Float|Max(Float) (- (Variables|Default|GetLocalSuspicion) (* DeltaTime (Variables|Default|GetSuspicionDrainRate))) 0.0) :!label _label))
                (if (and (<= _output_get_2 0.0) (Utilities|Enum|Equal(Enum) (Variables|Default|GetAlertLevel) "NewEnumerator1"))
                  (CallFunction|SetAlertedState "NewEnumerator0")))))
          (:Is%20Not%20Valid
            (goto _label))))
      (:then_1
        (switch Utilities|FlowControl|Switch|SwitchonEAlertState (Variables|Default|GetAlertLevel)
          (:NewEnumerator1
            (if _returnvalue :!label _label_2
              (if (or (Utilities|Enum|Equal(Enum) (Variables|/Game/Blueprints/BP_PlayerCharacter.BP_PlayerCharacter_C|GetCurrentIdentity _perceivedplayer_3) (Variables|/Game/Blueprints/BP_BitmaskGameMode.BP_BitmaskGameMode_C|GetLastPlayerIdentity (Variables|Default|GetBitmask%20Game%20Mode))) (Variables|/Game/Blueprints/BP_PlayerCharacter.BP_PlayerCharacter_C|GetIsTrespassing _perceivedplayer_3))
                (CallFunction|SetAlertedState "NewEnumerator3"))))
          (:NewEnumerator2
            (goto _label_2))
          (:NewEnumerator3
            (if (not _returnvalue)
              (CallFunction|SetAlertedState "NewEnumerator2"))))))))

(fn SetAlertedState
  (params (AlertLevel :type EAlertState%20Enum :default "NewEnumerator0"))
  (|CallParentFunction AlertLevel)
  (Variables|/Script/Engine.CharacterMovementComponent|SetMaxWalkSpeed (Variables|Character|GetCharacterMovement) (Utilities|Select :Index AlertLevel :NewEnumerator0 3e+02 :NewEnumerator1 3e+02 :NewEnumerator2 3.5e+02 :NewEnumerator3 4e+02 :NewEnumerator4 0.0 :NewEnumerator5 0.0))
  (switch Utilities|FlowControl|Switch|SwitchonEAlertState AlertLevel
    (:NewEnumerator2
      _)
    (:NewEnumerator3
      (if (Collision|IsOverlappingActor (Variables|Default|GetCaptureCapsule) (Variables|Default|GetPerceivedPlayer) :!class /Script/Engine.PrimitiveComponent)
        (CallFunction|Arrest))))
  (Variables|Default|SetLocalSuspicion (Variables|Default|GetMaxLocalSuspicion)))