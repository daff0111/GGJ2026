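; Base Blueprint for interaction stations that a player character with a matching identity can use.
; CanInteract checks the character's identity against the station's and rejects one blocked state.
; Start and stop calls set the interacting player, active flag and state enum, while Tick accumulates interaction time without completing anything itself.
; A separate reservation flag combines with the default state to report availability.
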(event EventBeginPlay)

(event Collision|EventActorBeginOverlap
  (params (OtherActor :type Actor%20Object%20Reference)))

(event EventTick
  (params (DeltaSeconds :type Float%20%28single-precision%29))
  (if (Variables|Default|GetInteractionActive)
    (Variables|Default|SetCurrentInteractionTime (+ DeltaSeconds (Variables|Default|GetCurrentInteractionTime)))))

(fn ConstructionScript)

(fn CanInteract
  (params (Character :type BP%20Player%20Character%20Object%20Reference))
  (return (and (Utilities|Enum|Equal(Enum) (Variables|/Game/Blueprints/BP_PlayerCharacter.BP_PlayerCharacter_C|GetCurrentIdentity Character) (Variables|Default|GetStationIdentity)) (Utilities|Enum|NotEqual(Enum) (Variables|Default|GetInteractionState) "NewEnumerator2"))))

(fn StartInteracting
  (params (PlayerCharacter :type BP%20Player%20Character%20Object%20Reference))
  (Utilities|IsValid PlayerCharacter
    (:Is%20Valid
      (Variables|Default|SetInteractingPlayer PlayerCharacter)
      (Variables|Default|SetInteractionActive true)
      (Variables|Default|SetCurrentInteractionTime 0.0)
      (CallFunction|SetInteractionState "NewEnumerator3"))))

(fn StopInteracting
  (Variables|Default|SetInteractingPlayer 0)
  (Variables|Default|SetInteractionActive false)
  (Variables|Default|SetCurrentInteractionTime 0.0)
  (CallFunction|SetInteractionState "NewEnumerator0"))

(fn SetInteractionState
  (params (InteractionState :type EInteractionStationState%20Enum :default "NewEnumerator0"))
  (Variables|Default|SetInteractionState InteractionState))

(fn SetIsReserved
  (params (IsReserved :type Boolean))
  (Variables|Default|SetIs%20Reserved IsReserved))

(fn IsAvailable
  (return (and (not (Variables|Default|GetIs%20Reserved)) (Utilities|Enum|Equal(Enum) (Variables|Default|GetInteractionState) "NewEnumerator0"))))