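; BP_EscapeZone is the exit trigger volume that wins the game when the player reaches it with the key.
; On box overlap, it casts the actor to BP_PlayerCharacter, checks HasKey, then calls WIN on BP_BitmaskGameMode.
; The construction script creates a dynamic material on the plane and scales its GridTile parameter from the actor's X scale so the tiling follows the zone's size.
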(event OnComponentBeginOverlap(Box)
  (params (OverlappedComponent :type Primitive%20Component%20Object%20Reference) (OtherActor :type Actor%20Object%20Reference) (OtherComp :type Primitive%20Component%20Object%20Reference) (OtherBodyIndex :type Integer) (bFromSweep :type Boolean) (SweepResult :type Hit%20Result%20Structure%20%28by%20ref%29))
  (bind _asbp_player_character (Utilities|Casting|CastToBP_PlayerCharacter OtherActor))
  (if (Variables|/Game/Blueprints/BP_PlayerCharacter.BP_PlayerCharacter_C|GetHasKey _asbp_player_character)
    (bind _asbp_bitmask_game_mode (Utilities|Casting|CastToBP_BitmaskGameMode (Game|GetGameMode)))
    (Default|WIN _asbp_bitmask_game_mode)))

(event EventBeginPlay)

(event Collision|EventActorBeginOverlap
  (params (OtherActor :type Actor%20Object%20Reference)))

(event EventTick
  (params (DeltaSeconds :type Float%20%28single-precision%29)))

(fn ConstructionScript
  (bind _returnvalue (Rendering|Material|CreateDynamicMaterialInstance (Variables|Default|GetPlane) 0 0 "None" :!class /Script/Engine.PrimitiveComponent))
  (Rendering|Material|SetScalarParameterValue _returnvalue "GridTile" (/ (.x (Transformation|GetActorScale3D)) 2.5) :!class /Script/Engine.MaterialInstanceDynamic))