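; Worker NPC that builds suspicion while it perceives the player in one specific identity.
; Each tick runs the parent logic, then raises local suspicion over time up to a cap, or drains it toward zero when no player is perceived or the identity differs.
; While suspicion sits at the cap and that identity is still perceived, it asks the Bitmask game mode to raise the alert level every tick.
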(event EventBeginPlay)

(event Collision|EventActorBeginOverlap
  (params (OtherActor :type Actor%20Object%20Reference)))

(event EventTick
  (params (DeltaSeconds :type Float%20%28single-precision%29))
  (|CallParentFunction DeltaSeconds)
  (CallFunction|UpdateWorkerSuspicion DeltaSeconds))

(fn ConstructionScript
  (|CallParentFunction))

(fn UpdateWorkerSuspicion
  (params (InputPin :type Float%20%28single-precision%29))
  (bind _perceivedplayer (Variables|Default|GetPerceivedPlayer))
  (bind _maxlocalsuspicion (Variables|Default|GetMaxLocalSuspicion))
  (Utilities|IsValid _perceivedplayer
    (:Is%20Valid
      (if (Utilities|Enum|Equal(Enum) (Variables|/Game/Blueprints/BP_PlayerCharacter.BP_PlayerCharacter_C|GetCurrentIdentity _perceivedplayer) "NewEnumerator0")
        (bind _output_get (Variables|Default|SetLocalSuspicion (Math|Float|Min(Float) (+ (Variables|Default|GetLocalSuspicion) (* InputPin (Variables|Default|GetSuspicionRaiseRate))) _maxlocalsuspicion)))
        (if (>= _output_get _maxlocalsuspicion)
          (Default|RaiseAlertLevel (Variables|Default|GetBitmask%20Game%20Mode) 1))
        (else
          (if (> (Variables|Default|GetLocalSuspicion) 0.0) :!label _label
            (Variables|Default|SetLocalSuspicion (Math|Float|Max(Float) (- (Variables|Default|GetLocalSuspicion) (* InputPin (Variables|Default|GetSuspicionDrainRate))) 0.0))))))
    (:Is%20Not%20Valid
      (goto _label))))